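; BP_Platform is a configurable platform for the platforming character that can double as a one-time checkpoint.
; Given a valid mesh, its construction script applies mesh and scale, showing Clouds instead of the mesh for checkpoints.
; When the character overlaps a checkpoint, it sets their respawn location above the platform and moves the nearest BP_OutOfBoundsBox below that point.
; It then clears the checkpoint flag.
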(event Collision|EventActorBeginOverlap
  (params (OtherActor :type Actor%20Object%20Reference))
  (if (Variables|Default|GetHasCheckpoint)
    (bind _asbp_platforming_character (Utilities|Casting|CastToBP_PlatformingCharacter OtherActor))
    (bind _output_get (Variables|/Game/Variant_Platforming/Blueprints/BP_PlatformingCharacter.BP_PlatformingCharacter_C|SetPlayerStartLocation _asbp_platforming_character (+ (Transformation|GetActorLocation) "0.000000,0.000000,250.000000")))
    (bind _outactors (Actor|GetAllActorsOfClass "/Game/Game/Meshes/Blueprints/BP_OutOfBoundsBox.BP_OutOfBoundsBox_C"))
    (Transformation|SetActorLocation (.ReturnValue (Actor|FindNearestActor _output_get _outactors)) (- _output_get "0.000000,0.000000,750.000000") false false)
    (Variables|Default|SetHasCheckpoint false)))

(fn ConstructionScript
  (bind _mesh (Variables|Default|Getmesh)
    (:then
      (Components|StaticMesh|SetStaticMesh (Variables|Default|GetStaticMesh) _mesh)
      (Transformation|SetWorldScale3D (Variables|Default|GetDefaultSceneRoot) (Math|Conversions|ToVector(Float) (Variables|Default|GetBoxScale)))
      (if (Variables|Default|GetHasCheckpoint)
        (Rendering|SetVisibility (Variables|Default|GetStaticMesh) false false)
        (Rendering|SetVisibility (Variables|Default|GetClouds) true false)
        (else
          (Rendering|SetVisibility (Variables|Default|GetStaticMesh) true false)
          (Rendering|SetVisibility (Variables|Default|GetClouds) false false))))
    (:else)))