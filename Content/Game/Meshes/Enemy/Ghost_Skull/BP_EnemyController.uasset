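; AI controller for BP_Enemy pawns that wanders at random and damages the player character on perception.
; A looping timer started on BeginPlay periodically moves the pawn to a random navigable point around its current location.
; Any perception update for BP_PlatformingCharacter, gained or lost, sets Attacking on controller and pawn and applies damage directly, with no range check.
; Nothing here clears Attacking or stops the wandering.
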(event OnTargetPerceptionUpdated(AIPerception)
  (params (Actor :type Actor%20Object%20Reference) (Stimulus :type AI%20Stimulus%20Structure))
  (bind _asbp_platforming_character (Utilities|Casting|CastToBP_PlatformingCharacter Actor))
  (bind _output_get (Variables|Default|SetAttacking true))
  (bind _asbp_enemy (Utilities|Casting|CastToBP_Enemy (Pawn|GetControlledPawn)))
  (Variables|/Game/Game/Meshes/Enemy/Ghost_Skull/BP_Enemy.BP_Enemy_C|SetAttacking _asbp_enemy _output_get)
  (Game|Damage|ApplyDamage _asbp_platforming_character 5.0 0 0))

(event Custom|OnMove
  (bind _asbp_enemy (Utilities|Casting|CastToBP_Enemy (Pawn|GetControlledPawn)))
  (bind _randomlocation (Class|NavigationSystemV1|GetRandomLocationinNavigableRadius (Transformation|GetActorLocation _asbp_enemy) 1e+03 (Variables|/Game/Game/Meshes/Enemy/Ghost_Skull/BP_Enemy.BP_Enemy_C|GetNavData _asbp_enemy) 0))
  (AI|AIMoveTo 0 _randomlocation 0 5.0 false))

(event EventBeginPlay
  (Utilities|Time|SetTimerbyEvent (delegate Custom|OnMove) 5.0 true))

(event Collision|EventActorBeginOverlap
  (params (OtherActor :type Actor%20Object%20Reference)))

(event EventTick
  (params (DeltaSeconds :type Float%20%28single-precision%29)))

(fn ConstructionScript)